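; AmberCharacter_BP is a character Blueprint that leaves surface-dependent stamps as it moves over sand or quicksand.
; Each character movement update with horizontal velocity calls SpawnStamp with the capsule's transform.
; SpawnStamp traces a short line downward and uses the hit physical material's surface type to select the sand or quicksand stamp actor to spawn, with no class set for the default surface.
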(event Custom|OnCharacterMovement
  (params (DeltaSeconds :type Float%20%28single-precision%29) (OldLocation :type Vector) (OldVelocity :type Vector))
  (if (> (Class|KismetMathLibrary|VSizeXYSquared (Variables|/Script/Engine.MovementComponent|GetVelocity (Variables|Character|GetCharacterMovement))) 0.0)
    (CallFunction|SpawnStamp (Transformation|GetWorldTransform (Variables|Default|GetCapsuleComponent)))))

(event EventBeginPlay
  (EventDispatchers|AssignOnCharacterMovementUpdated (delegate Custom|OnCharacterMovement)))

(fn ConstructionScript)

(fn SpawnStamp
  (params (StampTransform :type Transform))
  (bind _returnvalue (Transformation|GetActorLocation))
  (bind _outhit (Collision|LineTraceByChannel _returnvalue (+ _returnvalue "0, 0,-150.000000") "TraceTypeQuery1" false 0 "None"))
  (Utilities|IsValid (.PhysMat (Collision|BreakHitResult _outhit))
    (:Is%20Valid
      (Game|SpawnActorfromClass (Utilities|Select :Index (Variables|/Script/PhysicsCore.PhysicalMaterial|GetSurfaceType (.PhysMat (Collision|BreakHitResult _outhit))) :SurfaceType_Default 0 :SurfaceType1 "/Game/Blueprints/Stamps/SandStamp_BP.SandStamp_BP_C" :SurfaceType2 "/Game/Blueprints/Stamps/QuicksandStamp_BP.QuicksandStamp_BP_C") StampTransform "Undefined" 0 0))))