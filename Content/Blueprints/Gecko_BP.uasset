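; Gecko Blueprint that wanders to random nearby points while its IsNearPlayer flag is false.
; A looping timer started on BeginPlay fires Roam, which picks a random reachable point around the gecko's current location.
; A timeline turns the gecko toward that point on yaw only, then AIMoveTo sends it there once the turn finishes.
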(event Custom|Roam
  (bind _returnvalue (Transformation|GetActorLocation))
  ;[1 1 1] Roam
  (if (not (Variables|Default|GetisNearPlayer))
    (bind _output_get (Variables|Default|SetstartRotation (Transformation|GetActorRotation)))
    (bind _output_get_2 (Variables|Default|SetrandomLoc (.RandomLocation (AI|Navigation|GetRandomReachablePointinRadius _returnvalue 5e+02 0 0))))
    (bind _alpha (Timeline|Lerp_Timeline PlayFromStart)
      (:Update
        (Transformation|SetActorRotation (Math|Rotator|MakeRotator 0.0 0.0 (.Yaw (Math|Rotator|BreakRotator (Math|Rotator|Lerp(Rotator) _output_get (Math|Rotator|FindLookatRotation _returnvalue _output_get_2) _alpha))))))
      (:Finished
        (AI|AIMoveTo self (Variables|Default|GetrandomLoc) 0 5.0 false)))))

(event EventBeginPlay
  ;[1 1 1] Roam
  (Utilities|Time|SetTimerbyEvent (delegate Custom|Roam) 2.0 true))

(fn ConstructionScript)