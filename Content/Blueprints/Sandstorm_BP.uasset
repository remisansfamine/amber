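; Sandstorm actor that lays out Niagara effect emitters along a spline, draped onto the surface below or above it.
; The construction script steps along NiagaraSpline at EmitterDistance intervals and runs a tall vertical Visibility trace at each point.
; It adds a Niagara component at each impact point, offset from the actor's location, without checking whether the trace hit.
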(fn ConstructionScript
  (for _index (range 0 (Math|Float|Truncate (/ (Spline|GetSplineLength (Variables|Default|GetNiagaraSpline)) (Variables|Default|GetEmitterDistance))))
    (bind _outhit (Collision|LineTraceByChannel (Math|Vector|MakeVector (.x (Spline|GetLocationatDistanceAlongSpline (Variables|Default|GetNiagaraSpline) (* _index (Variables|Default|GetEmitterDistance)) "World")) (.y (Spline|GetLocationatDistanceAlongSpline (Variables|Default|GetNiagaraSpline) (* _index (Variables|Default|GetEmitterDistance)) "World")) 1e+05) (Math|Vector|MakeVector (.x (Spline|GetLocationatDistanceAlongSpline (Variables|Default|GetNiagaraSpline) (* _index (Variables|Default|GetEmitterDistance)) "World")) (.y (Spline|GetLocationatDistanceAlongSpline (Variables|Default|GetNiagaraSpline) (* _index (Variables|Default|GetEmitterDistance)) "World")) -1e+05) "TraceTypeQuery1" false 0 "None"))
    (AddComponent|AddNiagaraComponent false (Math|Conversions|ToTransform(Vector) (- (.impactpoint _outhit) (Transformation|GetActorLocation))))))